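; Enemy Blueprint, child of a parent enemy class, that fires a repeating three-shot volley along negative Y.
; Tick calls the parent, then runs a FireRate Delay, which ignores calls while pending and so acts as the fire timer.
; Each volley spawns BpprojectileEnemy2 at the Tope, Bet and Bott components with fixed damage and speed, then plays EnemyShot at the world origin.
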(event EventBeginPlay
  (|CallParentFunction))

(event Collision|EventActorBeginOverlap
  (params (OtherActor :type Actor%20Object%20Reference)))

(event EventTick
  (params (DeltaSeconds :type Float%20%28single-precision%29))
  (|CallParentFunction DeltaSeconds)
  (Utilities|FlowControl|Delay (Variables|Default|GetFireRate))
  (Game|SpawnActorfromClass "/Game/Blueprints/Projectiles/bpprojectileEnemy2.bpprojectileEnemy2_C" (Transformation|GetWorldTransform (Variables|Default|Gettope)) "AdjustIfPossibleButAlwaysSpawn" 0 1.0 "0.000000,-3000.000000,0.000000" "1.000000,1.000000,1.000000" 0)
  (Game|SpawnActorfromClass "/Game/Blueprints/Projectiles/bpprojectileEnemy2.bpprojectileEnemy2_C" (Transformation|GetWorldTransform (Variables|Default|Getbet)) "AdjustIfPossibleButAlwaysSpawn" 0 1.0 "0.000000,-3000.000000,0.000000" "1.000000,1.000000,1.000000" 0)
  (Game|SpawnActorfromClass "/Game/Blueprints/Projectiles/bpprojectileEnemy2.bpprojectileEnemy2_C" (Transformation|GetWorldTransform (Variables|Default|Getbott)) "AdjustIfPossibleButAlwaysSpawn" 0 1.0 "0.000000,-3000.000000,0.000000" "1.000000,1.000000,1.000000" 0)
  (Audio|PlaySoundatLocation "/Game/Audio/EnemyShot.EnemyShot" "0, 0, 0" "0, 0, 0" 1.0 1.0 0.0 0 0 0))

(fn ConstructionScript
  (|CallParentFunction))