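; Boss enemy Blueprint that repeatedly fires twin projectiles, building on its parent class's begin-play, tick and construction logic.
; A Delay on Tick, timed by FireRate, throttles firing without a separate timer.
; Each volley spawns two BpProjectileEnemy actors at the Top and Bottom components with a fixed damage and negative-Y speed.
; The EnemyShot sound plays at the world origin rather than at the boss.
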(event EventBeginPlay
  (|CallParentFunction))

(event EventTick
  (params (DeltaSeconds :type Float%20%28single-precision%29))
  (|CallParentFunction DeltaSeconds)
  (Utilities|FlowControl|Delay (Variables|Default|GetFireRate))
  (Game|SpawnActorfromClass "/Game/Blueprints/Projectiles/bpProjectileEnemy.bpProjectileEnemy_C" (Transformation|GetWorldTransform (Variables|Default|GetTop)) "AdjustIfPossibleButAlwaysSpawn" 0 5.0 "0.000000,-2000.000000,0.000000" "1.000000,1.000000,1.000000" 0)
  (Game|SpawnActorfromClass "/Game/Blueprints/Projectiles/bpProjectileEnemy.bpProjectileEnemy_C" (Transformation|GetWorldTransform (Variables|Default|GetBottom)) "AdjustIfPossibleButAlwaysSpawn" 0 5.0 "0.000000,-2000.000000,0.000000" "1.000000,1.000000,1.000000" 0)
  (Audio|PlaySoundatLocation "/Game/Audio/EnemyShot.EnemyShot" "0, 0, 0" "0, 0, 0" 1.0 1.0 0.0 0 0 0))

(fn ConstructionScript
  (|CallParentFunction))