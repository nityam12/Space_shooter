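; Special enemy variant that chases the player and fires enlarged projectiles on a repeating timer.
; Tick feeds a FireRate Delay, which spawns BpProjectileEnemy at ProjectileSpawn with fixed damage and Y-axis velocity, then plays the shot sound at world origin.
; Firing runs regardless of detection.
; PawnSensing casts any seen pawn to bpPlayer and issues AI Move To toward it.
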(event OnSeePawn(PawnSensing)
  (params (Pawn :type Pawn%20Object%20Reference))
  (bind _asbp_player (Utilities|Casting|CastTobpPlayer Pawn))
  (AI|AIMoveTo 0 "0, 0, 0" _asbp_player 5.0 false))

(event EventBeginPlay
  (|CallParentFunction))

(event EventTick
  (params (DeltaSeconds :type Float%20%28single-precision%29))
  (|CallParentFunction DeltaSeconds)
  (Utilities|FlowControl|Delay (Variables|Default|GetFireRate))
  (Game|SpawnActorfromClass "/Game/Blueprints/Projectiles/bpProjectileEnemy.bpProjectileEnemy_C" (Transformation|GetWorldTransform (Variables|Default|GetProjectileSpawn)) "Undefined" 0 1e+01 "0.000000,-2000.000000,0.000000" "2.000000,2.000000,2.000000" 0)
  (Audio|PlaySoundatLocation "/Game/Audio/EnemyShot.EnemyShot" "0, 0, 0" "0, 0, 0" 1.0 1.0 0.0 0 0 0))

(fn ConstructionScript
  (|CallParentFunction))